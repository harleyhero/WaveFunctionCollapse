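; Procedural map generator actor that runs Wave Function Collapse over a 3D grid of module templates on BeginPlay.
; It spawns hidden base modules, adds rotations for asymmetric ones, and creates instanced mesh components.
; Padding and depth limits prefilter each cell's possible modules before neighbours are linked.
; Tick-batched pending updates alternate with collapsing the lowest-option cell, though UpdateNode and PostCleanup are empty here.
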(event Custom|GenerateMap
  (bind _values (Utilities|Map|Values (Variables|WFC|Modules|GetMeshInstancers)))
  (for _array_element _values
    (Components|DestroyComponent _array_element))
  (Utilities|Map|Clear (Variables|WFC|Modules|GetMeshInstancers))
  (CallFunction|CreateBaseModuleInstances)
  (Utilities|FlowControl|DelayUntilNextTick)
  (CallFunction|InitGrid)
  (Utilities|FlowControl|DelayUntilNextTick)
  (CallFunction|InitNeighbours)
  (Utilities|FlowControl|DelayUntilNextTick)
  (CallFunction|IteratePendingNodes))

(event Custom|IterateWaveFunction
  (bind (_bcollapsed _nextcollapsenode) (CallFunction|CheckCollapsed))
  (Variables|WFC|GridState|SetNextCollapseNode _nextcollapsenode)
  (if _bcollapsed
    (CallFunction|PostCleanup)
    (else
      (CallFunction|CollapseNextNode))))

(event Custom|IteratePendingNodes
  (if (> (Utilities|Array|Length (Variables|WFC|GridState|GetPendingNodeUpdate)) 0)
    (CallFunction|UpdateNode (Utilities|Array|Get(acopy) (Variables|WFC|GridState|GetPendingNodeUpdate)))
    (Utilities|Array|RemoveIndex (Variables|WFC|GridState|GetPendingNodeUpdate))
    (if (< (Variables|WFC|GridState|GetCurrentNeighbourIter) (Variables|WFC|Settings|GetMaxNeighbourIter))
      (Math|Integer|IncrementInt (Variables|WFC|GridState|GetCurrentNeighbourIter)
        (:%20%20
          (CallFunction|IteratePendingNodes)))
      (else
        (Variables|WFC|GridState|SetCurrentNeighbourIter 0)
        (Utilities|FlowControl|DelayUntilNextTick)
        (CallFunction|IteratePendingNodes)))
    (else
      (Utilities|FlowControl|DelayUntilNextTick)
      (CallFunction|IterateWaveFunction))))

(event EventBeginPlay
  (CallFunction|GenerateMap))

(fn ConstructionScript)

(fn CreateBaseModuleInstances
  (for _array_element (Variables|WFC|Modules|GetModuleTemplates)
    (bind _returnvalue (Game|SpawnActorfromClass _array_element (Transformation|GetActorTransform) "Undefined" 0 0 0))
    (Utilities|Array|Add (Variables|WFC|Modules|GetBaseModules) _returnvalue)
    (Rendering|SetActorHiddenInGame _returnvalue true)
    (CallFunction|InitInstancedStaticMesh _returnvalue)
    (if (not (Default|CheckSymmetrical _returnvalue))
      (for _index (range 1 3)
        (bind _returnvalue_2 (Game|SpawnActorfromClass _array_element (Transformation|GetActorTransform) "Undefined" 0 _index 0))
        (Utilities|Array|Add (Variables|WFC|Modules|GetBaseModules) _returnvalue_2)
        (Default|RotateModule _returnvalue_2)
        (Rendering|SetActorHiddenInGame _returnvalue_2 true)))))

(fn InitGrid
  (bind _gridsize (Variables|WFC|Settings|GetGridSize))
  (bind _gridsize_2 (Variables|WFC|Settings|GetGridSize))
  (bind _gridsize_3 (Variables|WFC|Settings|GetGridSize))
  (bind _gridsize_4 (Variables|WFC|Settings|GetGridSize))
  (for _array_element (Variables|WFC|Modules|GetBaseModules)
    (LocalVariables|SetCurrentModule _array_element)
    (if (Math|Boolean|ANDBoolean (Utilities|Operators|EqualEqual :A (Variables|/Game/Blueprints/BP_WFCModule_Master.BP_WFCModule_Master_C|GetBotPadding _array_element) :ErrorTolerance 0.1) (Utilities|Operators|EqualEqual :A (Variables|/Game/Blueprints/BP_WFCModule_Master.BP_WFCModule_Master_C|GetTopPadding _array_element) :ErrorTolerance 0.1) (or (>= (+ (.x (Variables|/Game/Blueprints/BP_WFCModule_Master.BP_WFCModule_Master_C|GetBotMaxDepth _array_element)) (.x (Variables|/Game/Blueprints/BP_WFCModule_Master.BP_WFCModule_Master_C|GetTopMaxDepth _array_element))) (.x _gridsize)) (>= (+ (.y (Variables|/Game/Blueprints/BP_WFCModule_Master.BP_WFCModule_Master_C|GetBotMaxDepth _array_element)) (.y (Variables|/Game/Blueprints/BP_WFCModule_Master.BP_WFCModule_Master_C|GetTopMaxDepth _array_element))) (.y _gridsize))) (>= (+ (.z (Variables|/Game/Blueprints/BP_WFCModule_Master.BP_WFCModule_Master_C|GetBotMaxDepth _array_element)) (.z (Variables|/Game/Blueprints/BP_WFCModule_Master.BP_WFCModule_Master_C|GetTopMaxDepth _array_element))) (.z _gridsize)))
      (Utilities|Set|Add (LocalVariables|GetUnlimtedModules) (LocalVariables|GetCurrentModule))
      (else
        (if (Math|Boolean|ORBoolean (!= (.X (Math|Vector|BreakVector (Variables|/Game/Blueprints/BP_WFCModule_Master.BP_WFCModule_Master_C|GetBotPadding _array_element))) 0.0) (!= (.X (Math|Vector|BreakVector (Variables|/Game/Blueprints/BP_WFCModule_Master.BP_WFCModule_Master_C|GetTopPadding _array_element))) 0.0) (not (or (>= (+ (.x (Variables|/Game/Blueprints/BP_WFCModule_Master.BP_WFCModule_Master_C|GetBotMaxDepth _array_element)) (.x (Variables|/Game/Blueprints/BP_WFCModule_Master.BP_WFCModule_Master_C|GetTopMaxDepth _array_element))) (.x _gridsize)) (>= (+ (.y (Variables|/Game/Blueprints/BP_WFCModule_Master.BP_WFCModule_Master_C|GetBotMaxDepth _array_element)) (.y (Variables|/Game/Blueprints/BP_WFCModule_Master.BP_WFCModule_Master_C|GetTopMaxDepth _array_element))) (.y _gridsize)))))
          (Utilities|Set|Add (LocalVariables|GetXLimitedModules) (LocalVariables|GetCurrentModule)))
        (if (Math|Boolean|ORBoolean (!= (.Y (Math|Vector|BreakVector (Variables|/Game/Blueprints/BP_WFCModule_Master.BP_WFCModule_Master_C|GetBotPadding _array_element))) 0.0) (!= (.Y (Math|Vector|BreakVector (Variables|/Game/Blueprints/BP_WFCModule_Master.BP_WFCModule_Master_C|GetTopPadding _array_element))) 0.0) (not (or (>= (+ (.x (Variables|/Game/Blueprints/BP_WFCModule_Master.BP_WFCModule_Master_C|GetBotMaxDepth _array_element)) (.x (Variables|/Game/Blueprints/BP_WFCModule_Master.BP_WFCModule_Master_C|GetTopMaxDepth _array_element))) (.x _gridsize)) (>= (+ (.y (Variables|/Game/Blueprints/BP_WFCModule_Master.BP_WFCModule_Master_C|GetBotMaxDepth _array_element)) (.y (Variables|/Game/Blueprints/BP_WFCModule_Master.BP_WFCModule_Master_C|GetTopMaxDepth _array_element))) (.y _gridsize)))))
          (Utilities|Set|Add (LocalVariables|GetYLimitedModules) (LocalVariables|GetCurrentModule)))
        (if (Math|Boolean|ORBoolean (!= (.Z (Math|Vector|BreakVector (Variables|/Game/Blueprints/BP_WFCModule_Master.BP_WFCModule_Master_C|GetBotPadding _array_element))) 0.0) (!= (.Z (Math|Vector|BreakVector (Variables|/Game/Blueprints/BP_WFCModule_Master.BP_WFCModule_Master_C|GetTopPadding _array_element))) 0.0) (not (>= (+ (.z (Variables|/Game/Blueprints/BP_WFCModule_Master.BP_WFCModule_Master_C|GetBotMaxDepth _array_element)) (.z (Variables|/Game/Blueprints/BP_WFCModule_Master.BP_WFCModule_Master_C|GetTopMaxDepth _array_element))) (.z _gridsize))))
          (Utilities|Set|Add (LocalVariables|GetZLimitedModules) (LocalVariables|GetCurrentModule)))
        (Utilities|Set|Add (LocalVariables|GetLimitedModules) (LocalVariables|GetCurrentModule)))))
  (for _index (range 0 (- (Math|Float|Round (.z (Variables|WFC|Settings|GetGridSize))) 1))
    (LocalVariables|SetZIndex _index)
    (Utilities|Set|Clear (LocalVariables|GetZEliminatedModules))
    (bind _result (Utilities|Set|ToArray (LocalVariables|GetZLimitedModules)))
    (for _array_element_2 _result
      (if (Math|Boolean|ORBoolean (< (LocalVariables|GetZIndex) (.z (Variables|/Game/Blueprints/BP_WFCModule_Master.BP_WFCModule_Master_C|GetBotPadding _array_element_2))) (>= (LocalVariables|GetZIndex) (- (.z _gridsize_2) (.z (Variables|/Game/Blueprints/BP_WFCModule_Master.BP_WFCModule_Master_C|GetTopPadding _array_element_2)))) (and (>= (LocalVariables|GetZIndex) (.z (Variables|/Game/Blueprints/BP_WFCModule_Master.BP_WFCModule_Master_C|GetBotMaxDepth _array_element_2))) (< (LocalVariables|GetZIndex) (- (.z _gridsize_2) (.z (Variables|/Game/Blueprints/BP_WFCModule_Master.BP_WFCModule_Master_C|GetTopMaxDepth _array_element_2))))))
        (Utilities|Set|Add (LocalVariables|GetZEliminatedModules) _array_element_2)))
    (for _index_2 (range 0 (- (Math|Float|Round (.y (Variables|WFC|Settings|GetGridSize))) 1))
      (LocalVariables|SetYIndex _index_2)
      (Utilities|Set|Clear (LocalVariables|GetYEliminatedModules))
      (bind _result_2 (Utilities|Set|Difference (LocalVariables|GetYLimitedModules) (LocalVariables|GetZEliminatedModules)))
      (bind _result_3 (Utilities|Set|ToArray _result_2))
      (for _array_element_3 _result_3
        (if (Math|Boolean|ORBoolean (< (LocalVariables|GetYIndex) (.y (Variables|/Game/Blueprints/BP_WFCModule_Master.BP_WFCModule_Master_C|GetBotPadding _array_element_3))) (>= (LocalVariables|GetYIndex) (- (.y _gridsize_3) (.y (Variables|/Game/Blueprints/BP_WFCModule_Master.BP_WFCModule_Master_C|GetTopPadding _array_element_3)))) (Math|Boolean|ANDBoolean (== (.x (Variables|/Game/Blueprints/BP_WFCModule_Master.BP_WFCModule_Master_C|GetBotMaxDepth _array_element_3)) 0.0) (>= (LocalVariables|GetYIndex) (.y (Variables|/Game/Blueprints/BP_WFCModule_Master.BP_WFCModule_Master_C|GetBotMaxDepth _array_element_3))) (< (LocalVariables|GetYIndex) (- (.y _gridsize_3) (.y (Variables|/Game/Blueprints/BP_WFCModule_Master.BP_WFCModule_Master_C|GetTopMaxDepth _array_element_3)))) (== (.x (Variables|/Game/Blueprints/BP_WFCModule_Master.BP_WFCModule_Master_C|GetTopMaxDepth _array_element_3)) 0.0)))
          (Utilities|Set|Add (LocalVariables|GetYEliminatedModules) _array_element_3)))
      (for _index_3 (range 0 (- (Math|Float|Round (.x (Variables|WFC|Settings|GetGridSize))) 1))
        (LocalVariables|SetXIndex _index_3)
        (Utilities|Set|Clear (LocalVariables|GetXEliminatedModules))
        (bind _result_4 (Utilities|Set|Union (LocalVariables|GetYEliminatedModules) (LocalVariables|GetZEliminatedModules)))
        (bind _result_5 (Utilities|Set|Difference (LocalVariables|GetXLimitedModules) _result_4))
        (bind _result_6 (Utilities|Set|ToArray _result_5))
        (for _array_element_4 _result_6
          (if (Math|Boolean|ORBoolean (< (LocalVariables|GetXIndex) (.x (Variables|/Game/Blueprints/BP_WFCModule_Master.BP_WFCModule_Master_C|GetBotPadding _array_element_4))) (>= (LocalVariables|GetXIndex) (- (.x _gridsize_4) (.x (Variables|/Game/Blueprints/BP_WFCModule_Master.BP_WFCModule_Master_C|GetTopPadding _array_element_4)))) (Math|Boolean|ANDBoolean (< (LocalVariables|GetXIndex) (- (.x _gridsize_4) (.x (Variables|/Game/Blueprints/BP_WFCModule_Master.BP_WFCModule_Master_C|GetTopMaxDepth _array_element_4)))) (>= (LocalVariables|GetXIndex) (.x (Variables|/Game/Blueprints/BP_WFCModule_Master.BP_WFCModule_Master_C|GetBotMaxDepth _array_element_4))) (< (LocalVariables|GetYIndex) (- (.y _gridsize_4) (.y (Variables|/Game/Blueprints/BP_WFCModule_Master.BP_WFCModule_Master_C|GetTopMaxDepth _array_element_4)))) (>= (LocalVariables|GetYIndex) (.y (Variables|/Game/Blueprints/BP_WFCModule_Master.BP_WFCModule_Master_C|GetBotMaxDepth _array_element_4)))))
            (Utilities|Set|Add (LocalVariables|GetXEliminatedModules) _array_element_4)))
        (bind _result_7 (Utilities|Set|Union _result_4 (LocalVariables|GetXEliminatedModules)))
        (bind _result_8 (Utilities|Set|Difference (LocalVariables|GetLimitedModules) _result_7))
        (bind _result_9 (Utilities|Set|Union _result_8 (LocalVariables|GetUnlimtedModules)))
        (bind _result_10 (Utilities|Set|ToArray _result_9))
        (bind _returnvalue (Game|ConstructObjectfromClass "/Game/Blueprints/BP_WFCNodeData.BP_WFCNodeData_C"))
        (Default|SetPossibleModules _returnvalue _result_10)
        (bind _output_get (Variables|/Game/Blueprints/BP_WFCNodeData.BP_WFCNodeData_C|SetGridPosition _returnvalue (Math|Vector|MakeVector (Math|Conversions|ToFloat(Integer) (LocalVariables|GetXIndex)) (Math|Conversions|ToFloat(Integer) (LocalVariables|GetYIndex)) (Math|Conversions|ToFloat(Integer) (LocalVariables|GetZIndex)))))
        (Utilities|Map|Add (Variables|WFC|GridState|GetGridData) _output_get _returnvalue)
        (Utilities|Array|Add (Variables|WFC|GridState|GetPendingNodeUpdate) _returnvalue)
        (if (Variables|WFC|Settings|GetbDebugText)
          (bind _returnvalue_2 (Game|SpawnActorfromClass "/Script/Engine.TextRenderActor" (Math|Transform|MakeTransform (+ (* (Math|Vector|MakeVector (Math|Conversions|ToFloat(Integer) (LocalVariables|GetXIndex)) (Math|Conversions|ToFloat(Integer) (LocalVariables|GetYIndex)) (Math|Conversions|ToFloat(Integer) (LocalVariables|GetZIndex))) (Variables|WFC|Settings|GetGridScale)) (Transformation|GetActorLocation)) "0, 0, 0" "1.000000,1.000000,1.000000") "Undefined" 0 0))
          (Utilities|Map|Add (Variables|WFC|GridState|GetDebugText) (Math|Vector|MakeVector (Math|Conversions|ToFloat(Integer) (LocalVariables|GetXIndex)) (Math|Conversions|ToFloat(Integer) (LocalVariables|GetYIndex)) (Math|Conversions|ToFloat(Integer) (LocalVariables|GetZIndex))) _returnvalue_2)
          (CallFunction|UpdateDebugText (Math|Vector|MakeVector (Math|Conversions|ToFloat(Integer) (LocalVariables|GetXIndex)) (Math|Conversions|ToFloat(Integer) (LocalVariables|GetYIndex)) (Math|Conversions|ToFloat(Integer) (LocalVariables|GetZIndex))))
          (Rendering|Components|TextRender|SetWorldSize (Variables|/Script/Engine.TextRenderActor|GetTextRender _returnvalue_2) (Variables|WFC|Settings|GetDebugTextSize))
          (Rendering|Components|TextRender|SetTextRenderColor (Variables|/Script/Engine.TextRenderActor|GetTextRender _returnvalue_2) (Variables|WFC|Settings|GetDebugTextColor))
          (Class|TextRenderComponent|SetVerticalAlignment (Variables|/Script/Engine.TextRenderActor|GetTextRender _returnvalue_2) "EVRTA_TextCenter")
          (Rendering|Components|TextRender|SetHorizontalAlignment (Variables|/Script/Engine.TextRenderActor|GetTextRender _returnvalue_2) "EHTA_Center"))))))

(fn UpdateDebugText
  (params (InGridPosition :type Vector))
  (for _array_element (Variables|/Game/Blueprints/BP_WFCNodeData.BP_WFCNodeData_C|GetPossibleModules (.Value (Utilities|Map|Find (Variables|WFC|GridState|GetGridData) InGridPosition)))
    (LocalVariables|SetNewDebugText (Utilities|String|Append (LocalVariables|GetNewDebugText) " 
" (Utilities|GetDisplayName _array_element))))
  (Rendering|Components|TextRender|SetText (Variables|/Script/Engine.TextRenderActor|GetTextRender (.Value (Utilities|Map|Find (Variables|WFC|GridState|GetDebugText) InGridPosition))) (Utilities|Text|ToText(String) (LocalVariables|GetNewDebugText))))

(fn InitNeighbours
  (bind _values (Utilities|Map|Values (Variables|WFC|GridState|GetGridData)))
  (for _array_element _values
    (CallFunction|SetNeighbors (Variables|/Game/Blueprints/BP_WFCNodeData.BP_WFCNodeData_C|GetGridPosition _array_element) _array_element)))

(fn SetNeighbors
  (params (InPosition :type Vector) (InNodeData :type BP%20WFC%20Node%20Data%20Object%20Reference))
  (bind (_x _y _z) (Math|Vector|BreakVector InPosition))
  (bind _gridsize (Variables|WFC|Settings|GetGridSize))
  (bind _returnvalue (- _gridsize 1))
  (if (== (.x _returnvalue) _x)
    _
    (else
      (Variables|/Game/Blueprints/BP_WFCNodeData.BP_WFCNodeData_C|SetPosXNeighbour InNodeData (.Value (Utilities|Map|Find (Variables|WFC|GridState|GetGridData) (+ InPosition "1.000000,0.000000,0.000000"))))))
  (if (== (.y _returnvalue) _y)
    _
    (else
      (Variables|/Game/Blueprints/BP_WFCNodeData.BP_WFCNodeData_C|SetPosYNeighbour InNodeData (.Value (Utilities|Map|Find (Variables|WFC|GridState|GetGridData) (+ InPosition "0.000000,1.000000,0.000000"))))))
  (if (== (.z _returnvalue) _z)
    _
    (else
      (Variables|/Game/Blueprints/BP_WFCNodeData.BP_WFCNodeData_C|SetPosZNeighbour InNodeData (.Value (Utilities|Map|Find (Variables|WFC|GridState|GetGridData) (+ InPosition "0.000000,0.000000,1.000000"))))))
  (if (== (.x InPosition) 0.0)
    _
    (else
      (Variables|/Game/Blueprints/BP_WFCNodeData.BP_WFCNodeData_C|SetNegXNeighbour InNodeData (.Value (Utilities|Map|Find (Variables|WFC|GridState|GetGridData) (+ InPosition "-1.000000,0.000000,0.000000"))))))
  (if (== (.y InPosition) 0.0)
    _
    (else
      (Variables|/Game/Blueprints/BP_WFCNodeData.BP_WFCNodeData_C|SetNegYNeighbour InNodeData (.Value (Utilities|Map|Find (Variables|WFC|GridState|GetGridData) (+ InPosition "0.000000,-1.000000,0.000000"))))))
  (if (not (== (.z InPosition) 0.0))
    (Variables|/Game/Blueprints/BP_WFCNodeData.BP_WFCNodeData_C|SetNegZNeighbour InNodeData (.Value (Utilities|Map|Find (Variables|WFC|GridState|GetGridData) (+ InPosition "0.000000,0.000000,-1.000000"))))))

(fn CheckCollapsed
  (bind _values (Utilities|Map|Values (Variables|WFC|GridState|GetGridData)))
  (for _array_element _values
    (if (> (Utilities|Array|Length (Variables|/Game/Blueprints/BP_WFCNodeData.BP_WFCNodeData_C|GetPossibleModules _array_element)) 1)
      (LocalVariables|SetbAllCollapsed false)
      (if (< (Utilities|Array|Length (Variables|/Game/Blueprints/BP_WFCNodeData.BP_WFCNodeData_C|GetPossibleModules _array_element)) (LocalVariables|GetCurrentLowest))
        (LocalVariables|SetCurrentLowest (Utilities|Array|Length (Variables|/Game/Blueprints/BP_WFCNodeData.BP_WFCNodeData_C|GetPossibleModules _array_element)))
        (LocalVariables|SetCurrentNextNode _array_element))))
  (return (LocalVariables|GetbAllCollapsed) (LocalVariables|GetCurrentNextNode)))

(fn PostCleanup)

(fn CollapseNextNode
  (bind _nextcollapsenode (Variables|WFC|GridState|GetNextCollapseNode))
  (if (Variables|/Game/Blueprints/BP_WFCNodeData.BP_WFCNodeData_C|GetbNodeInitialised _nextcollapsenode)
    _
    (else
      (Default|InitNode _nextcollapsenode)))
  (Default|CollapseNode _nextcollapsenode)
  (if (Variables|WFC|Settings|GetbDebugText)
    (CallFunction|UpdateDebugText (Variables|/Game/Blueprints/BP_WFCNodeData.BP_WFCNodeData_C|GetGridPosition _nextcollapsenode)))
  (CallFunction|IteratePendingNodes))

(fn UpdateNode
  (params (InNodeData :type BP%20WFC%20Node%20Data%20Object%20Reference)))

(fn InitInstancedStaticMesh
  (params (InModule :type BP%20WFC%20Module%20Master%20Object%20Reference))
  (bind _allstaticmeshes (Default|GetAllStaticMeshes InModule))
  (for _array_element _allstaticmeshes
    (if (not (Utilities|Map|Contains (Variables|WFC|Modules|GetMeshInstancers) (Utilities|GetDisplayName _array_element)))
      (bind _returnvalue (AddComponent|AddInstancedStaticMeshComponent false))
      (Components|StaticMesh|SetStaticMesh _returnvalue (Variables|/Script/Engine.StaticMeshComponent|GetStaticMesh _array_element))
      (Utilities|Map|Add (Variables|WFC|Modules|GetMeshInstancers) (Utilities|GetDisplayName (Variables|/Script/Engine.StaticMeshComponent|GetStaticMesh _array_element)) _returnvalue))))