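; Data for one Wave Function Collapse node, holding its candidate modules and neighbour references in six axis directions.
; InitNode caches possible sockets per direction and builds direction-to-socket-to-module lookup objects.
; RemoveInvalidPossibilities uses those lookups to remove modules matching an invalid socket, subtracting their weights from the total without refreshing the socket caches.
; CollapseNode picks one module by weighted random selection, then refreshes the socket caches.
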(fn SetPossibleModules
  (params (NewPossibilities :type Array%20of%20BP%20WFC%20Module%20Master%20Object%20References))
  (Variables|State|SetPossibleModules NewPossibilities)
  (Variables|State|SetbWeightsSet false))

(fn InitNode
  (CallFunction|UpdatePossibleSockets)
  (CallFunction|SetupSocketMap)
  (Variables|State|SetbNodeInitialised true))

(fn UpdatePossibleSockets
  (Utilities|Set|Clear (Variables|Sockets|GetPossiblePosXSockets))
  (Utilities|Set|Clear (Variables|Sockets|GetPossibleNegXSockets))
  (Utilities|Set|Clear (Variables|Sockets|GetPossiblePosYSockets))
  (Utilities|Set|Clear (Variables|Sockets|GetPossibleNegYSockets))
  (Utilities|Set|Clear (Variables|Sockets|GetPossiblePosZSockets))
  (Utilities|Set|Clear (Variables|Sockets|GetPossibleNegZSockets))
  (for _array_element (Variables|State|GetPossibleModules)
    (bind _output_get (LocalVariables|SetCurrentModule _array_element))
    (Utilities|Set|Add (Variables|Sockets|GetPossiblePosXSockets) (Default|GetSocketValue _output_get "NewEnumerator0"))
    (Utilities|Set|Add (Variables|Sockets|GetPossibleNegXSockets) (Default|GetSocketValue _output_get "NewEnumerator1"))
    (Utilities|Set|Add (Variables|Sockets|GetPossiblePosYSockets) (Default|GetSocketValue _output_get "NewEnumerator2"))
    (Utilities|Set|Add (Variables|Sockets|GetPossibleNegYSockets) (Default|GetSocketValue _output_get "NewEnumerator3"))
    (Utilities|Set|Add (Variables|Sockets|GetPossiblePosZSockets) (Default|GetSocketValue _output_get "NewEnumerator4"))
    (Utilities|Set|Add (Variables|Sockets|GetPossibleNegZSockets) (Default|GetSocketValue _output_get "NewEnumerator5"))))

(fn SetupSocketMap
  (for _array_element (Variables|State|GetPossibleModules)
    (bind _output_get (LocalVariables|SetCurrentModule _array_element))
    (CallFunction|AddtoSocketMap "NewEnumerator0" (Default|GetSocketValue _output_get "NewEnumerator0") (LocalVariables|GetCurrentModule))
    (CallFunction|AddtoSocketMap "NewEnumerator1" (Default|GetSocketValue (LocalVariables|GetCurrentModule) "NewEnumerator1") (LocalVariables|GetCurrentModule))
    (CallFunction|AddtoSocketMap "NewEnumerator2" (Default|GetSocketValue (LocalVariables|GetCurrentModule) "NewEnumerator2") (LocalVariables|GetCurrentModule))
    (CallFunction|AddtoSocketMap "NewEnumerator3" (Default|GetSocketValue (LocalVariables|GetCurrentModule) "NewEnumerator3") (LocalVariables|GetCurrentModule))
    (CallFunction|AddtoSocketMap "NewEnumerator4" (Default|GetSocketValue (LocalVariables|GetCurrentModule) "NewEnumerator4") (LocalVariables|GetCurrentModule))
    (CallFunction|AddtoSocketMap "NewEnumerator5" (Default|GetSocketValue (LocalVariables|GetCurrentModule) "NewEnumerator5") (LocalVariables|GetCurrentModule))))

(fn CollapseNode
  (if (Variables|State|GetbWeightsSet)
    _
    (else
      (Variables|State|SetTotalWeights 0.0)
      (for _array_element (Variables|State|GetPossibleModules)
        (Variables|State|SetTotalWeights (+ (Variables|State|GetTotalWeights) (Variables|/Game/Blueprints/BP_WFCModule_Master.BP_WFCModule_Master_C|GetWeight _array_element))))
      (Variables|State|SetbWeightsSet true)))
  (LocalVariables|SetRandValue (Math|Random|RandomFloatinRange 0.0 (Variables|State|GetTotalWeights)))
  (for _array_element_2 (Variables|State|GetPossibleModules)
    (bind _output_get (LocalVariables|SetWeightTally (+ (Variables|/Game/Blueprints/BP_WFCModule_Master.BP_WFCModule_Master_C|GetWeight _array_element_2) (LocalVariables|GetWeightTally))))
    (if (<= (LocalVariables|GetRandValue) _output_get)
      (CallFunction|SetPossibleModules (Utilities|Array|MakeArray _array_element_2))
      (CallFunction|UpdatePossibleSockets)
      (return))))

(fn GetValidNeighbours
  (Utilities|FlowControl|Sequence
    (:then_0
      (bind _posxneighbour (Variables|Nodes|GetPosXNeighbour)
        (:then
          (Utilities|Map|Add (LocalVariables|GetValidNeighbours) "NewEnumerator0" _posxneighbour))
        (:else)))
    (:then_1
      (bind _negxneighbour (Variables|Nodes|GetNegXNeighbour)
        (:then
          (Utilities|Map|Add (LocalVariables|GetValidNeighbours) "NewEnumerator1" _negxneighbour))
        (:else)))
    (:then_2
      (bind _posyneighbour (Variables|Nodes|GetPosYNeighbour)
        (:then
          (Utilities|Map|Add (LocalVariables|GetValidNeighbours) "NewEnumerator2" _posyneighbour))
        (:else)))
    (:then_3
      (bind _negyneighbour (Variables|Nodes|GetNegYNeighbour)
        (:then
          (Utilities|Map|Add (LocalVariables|GetValidNeighbours) "NewEnumerator3" _negyneighbour))
        (:else)))
    (:then_4
      (bind _poszneighbour (Variables|Nodes|GetPosZNeighbour)
        (:then
          (Utilities|Map|Add (LocalVariables|GetValidNeighbours) "NewEnumerator4" _poszneighbour))
        (:else)))
    (:then_5
      (bind _negzneighbour (Variables|Nodes|GetNegZNeighbour)
        (:then
          (Utilities|Map|Add (LocalVariables|GetValidNeighbours) "NewEnumerator5" _negzneighbour))
        (:else)))
    (:then_6
      (return (LocalVariables|GetValidNeighbours)))))

(fn GetPossibleSockets
  (params (InDirection :type EWFCSocketDirection%20Enum :default "NewEnumerator0"))
  (return (Utilities|Select :Index InDirection :NewEnumerator0 (Variables|Sockets|GetPossiblePosXSockets) :NewEnumerator1 (Variables|Sockets|GetPossibleNegXSockets) :NewEnumerator2 (Variables|Sockets|GetPossiblePosYSockets) :NewEnumerator3 (Variables|Sockets|GetPossibleNegYSockets) :NewEnumerator4 (Variables|Sockets|GetPossiblePosZSockets) :NewEnumerator5 (Variables|Sockets|GetPossibleNegZSockets))))

(fn RemoveInvalidPossibilities
  (params (InSocketDirection :type EWFCSocketDirection%20Enum :default "NewEnumerator0") (InInvalidSocket :type EWFC_SocketNames%20Enum :default "NewEnumerator30"))
  (bind _posxsocketdata (Variables|Sockets|GetPosXSocketData))
  (bind _negxsocketdata (Variables|Sockets|GetNegXSocketData))
  (bind _posysocketdata (Variables|Sockets|GetPosYSocketData))
  (bind _negysocketdata (Variables|Sockets|GetNegYSocketData))
  (bind _poszsocketdata (Variables|Sockets|GetPosZSocketData))
  (bind _negzsocketdata (Variables|Sockets|GetNegZSocketData))
  (bind _returnvalue (Utilities|Select :Index InSocketDirection :NewEnumerator0 _posxsocketdata :NewEnumerator1 _negxsocketdata :NewEnumerator2 _posysocketdata :NewEnumerator3 _negysocketdata :NewEnumerator4 _poszsocketdata :NewEnumerator5 _negzsocketdata))
  (Utilities|IsValid _returnvalue
    (:Is%20Valid
      (for _array_element (Variables|/Game/Blueprints/BP_WFCNodeSocketModuleData.BP_WFCNodeSocketModuleData_C|GetModules (.Value (Utilities|Map|Find (Variables|/Game/Blueprints/BP_WFCNodeSocketData.BP_WFCNodeSocketData_C|GetSocketModuleData _returnvalue) InInvalidSocket)))
        (bind _returnvalue_2 (Utilities|Array|RemoveItem (Variables|State|GetPossibleModules) _array_element))
        (if _returnvalue_2
          (Variables|State|SetTotalWeights (- (Variables|State|GetTotalWeights) (Variables|/Game/Blueprints/BP_WFCModule_Master.BP_WFCModule_Master_C|GetWeight _array_element))))))))

(fn AddtoSocketMap
  (params (InDirection :type EWFCSocketDirection%20Enum :default "NewEnumerator0") (InSocket :type EWFC_SocketNames%20Enum :default "NewEnumerator30") (InModule :type BP%20WFC%20Module%20Master%20Object%20Reference))
  (bind _posxsocketdata (Variables|Sockets|GetPosXSocketData))
  (bind _negxsocketdata (Variables|Sockets|GetNegXSocketData))
  (bind _posysocketdata (Variables|Sockets|GetPosYSocketData))
  (bind _negysocketdata (Variables|Sockets|GetNegYSocketData))
  (bind _poszsocketdata (Variables|Sockets|GetPosZSocketData))
  (bind _negzsocketdata (Variables|Sockets|GetNegZSocketData))
  (bind _returnvalue (Utilities|Select :Index InDirection :NewEnumerator0 _posxsocketdata :NewEnumerator1 _negxsocketdata :NewEnumerator2 _posysocketdata :NewEnumerator3 _negysocketdata :NewEnumerator4 _poszsocketdata :NewEnumerator5 _negzsocketdata))
  (bind _socketmoduledata (Variables|/Game/Blueprints/BP_WFCNodeSocketData.BP_WFCNodeSocketData_C|GetSocketModuleData _returnvalue))
  (bind (_value _returnvalue_2) (Utilities|Map|Find _socketmoduledata InSocket))
  (Utilities|IsValid _returnvalue
    (:Is%20Valid
      _)
    (:Is%20Not%20Valid
      (bind _returnvalue_3 (Game|ConstructObjectfromClass "/Game/Blueprints/BP_WFCNodeSocketData.BP_WFCNodeSocketData_C"))
      (|SetBy-RefVar _returnvalue _returnvalue_3)))
  (if _returnvalue_2
    (Utilities|Array|Add (Variables|/Game/Blueprints/BP_WFCNodeSocketModuleData.BP_WFCNodeSocketModuleData_C|GetModules _value) InModule)
    (else
      (bind _returnvalue_4 (Game|ConstructObjectfromClass "/Game/Blueprints/BP_WFCNodeSocketModuleData.BP_WFCNodeSocketModuleData_C"))
      (Utilities|Array|Add (Variables|/Game/Blueprints/BP_WFCNodeSocketModuleData.BP_WFCNodeSocketModuleData_C|GetModules _returnvalue_4) InModule)
      (Utilities|Map|Add _socketmoduledata InSocket _returnvalue_4))))