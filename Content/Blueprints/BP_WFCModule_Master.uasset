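; Wave Function Collapse module Blueprint with a mesh and six socket enums, each shown on a text label.
; RotateModule yaws the mesh by RotationIndex quarter turns, shifts side sockets from their construction-time order, and rotates every socket's variant.
; RotateSocket parses the enum name, increments its numeric suffix modulo 4 (S stays fixed), and looks up the result in a construction-built name-to-enum map.
; CheckSymmetrical detects rotationally symmetric modules.
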(event Custom|RotateModule
  (bind _rotationindex (Variables|WFC|GetRotationIndex))
  (bind _startsockets (Variables|Default|GetStartSockets))
  (Transformation|AddLocalRotation (Variables|Default|GetStaticMesh) (Math|Rotator|MakeRotator 0.0 0.0 (Math|Conversions|ToFloat(Integer) (* _rotationindex 90))) false false)
  (Variables|WFC|Sockets|SetPosXSocket (CallFunction|RotateSocket (Utilities|Array|Get(acopy) _startsockets (Math|Integer|%(Integer) _rotationindex 4)) _rotationindex))
  (Variables|WFC|Sockets|SetPosYSocket (CallFunction|RotateSocket (Utilities|Array|Get(acopy) _startsockets (Math|Integer|%(Integer) (+ _rotationindex 3) 4)) _rotationindex))
  (Variables|WFC|Sockets|SetNegXSocket (CallFunction|RotateSocket (Utilities|Array|Get(acopy) _startsockets (Math|Integer|%(Integer) (+ _rotationindex 2) 4)) _rotationindex))
  (Variables|WFC|Sockets|SetNegYSocket (CallFunction|RotateSocket (Utilities|Array|Get(acopy) _startsockets (Math|Integer|%(Integer) (+ _rotationindex 1) 4)) _rotationindex))
  (Variables|WFC|Sockets|SetPosZSocket (CallFunction|RotateSocket (Variables|WFC|Sockets|GetPosZSocket) _rotationindex))
  (Variables|WFC|Sockets|SetNegZSocket (CallFunction|RotateSocket (Variables|WFC|Sockets|GetNegZSocket) _rotationindex))
  (CallFunction|UpdateDisplayText))

(fn ConstructionScript
  (Utilities|Map|Clear (Variables|WFC|Sockets|GetSocketMap))
  (bind _enumvalue (|ForEachEWFC_SocketNames)
    (:LoopBody
      (Utilities|Map|Add (Variables|WFC|Sockets|GetSocketMap) (Utilities|String|EnumtoString _enumvalue) _enumvalue))
    (:then
      (Variables|Default|SetStartSockets (Utilities|Array|MakeArray (Variables|WFC|Sockets|GetPosXSocket) (Variables|WFC|Sockets|GetNegYSocket) (Variables|WFC|Sockets|GetNegXSocket) (Variables|WFC|Sockets|GetPosYSocket)))
      (CallFunction|UpdateDisplayText))))

(fn UpdateDisplayText
  (Rendering|Components|TextRender|SetText (Variables|Default|GetPosXText) (Utilities|Text|ToText(String) (Utilities|String|EnumtoString (Variables|WFC|Sockets|GetPosXSocket))))
  (Rendering|Components|TextRender|SetText (Variables|Default|GetNegXText) (Utilities|Text|ToText(String) (Utilities|String|EnumtoString (Variables|WFC|Sockets|GetNegXSocket))))
  (Rendering|Components|TextRender|SetText (Variables|Default|GetPosYText) (Utilities|Text|ToText(String) (Utilities|String|EnumtoString (Variables|WFC|Sockets|GetPosYSocket))))
  (Rendering|Components|TextRender|SetText (Variables|Default|GetNegYText) (Utilities|Text|ToText(String) (Utilities|String|EnumtoString (Variables|WFC|Sockets|GetNegYSocket))))
  (Rendering|Components|TextRender|SetText (Variables|Default|GetPosZText) (Utilities|Text|ToText(String) (Utilities|String|EnumtoString (Variables|WFC|Sockets|GetPosZSocket))))
  (Rendering|Components|TextRender|SetText (Variables|Default|GetNegZText) (Utilities|Text|ToText(String) (Utilities|String|EnumtoString (Variables|WFC|Sockets|GetNegZSocket)))))

(fn RotateSocket
  (params (InSocket :type EWFC_SocketNames%20Enum :default "NewEnumerator0") (RotationIndex :type Integer))
  (bind _returnvalue (Utilities|String|EnumtoString InSocket))
  (bind _returnvalue_2 (Utilities|String|ParseIntoArray _returnvalue "_"))
  (bind _output (Utilities|Array|Get(acopy) _returnvalue_2 2))
  (switch string _output
    (:Default
      (return (.Value (Utilities|Map|Find (Variables|WFC|Sockets|GetSocketMap) (Utilities|String|Append (Utilities|Array|Get(acopy) _returnvalue_2) "_" (Utilities|Array|Get(acopy) _returnvalue_2 1) "_" (Utilities|String|ToString(Integer) (Math|Integer|%(Integer) (+ (Math|Conversions|ToInteger(Byte) _output) RotationIndex) 4)))))))
    (:S
      (return InSocket))))

(fn CheckSymmetrical
  (bind _negxsocket (Variables|WFC|Sockets|GetNegXSocket))
  (bind _posysocket (Variables|WFC|Sockets|GetPosYSocket))
  (return (Math|Boolean|ANDBoolean (Utilities|Enum|Equal(Enum) (Variables|WFC|Sockets|GetPosXSocket) _negxsocket) (Utilities|Enum|Equal(Enum) _negxsocket _posysocket) (Utilities|Enum|Equal(Enum) _posysocket (Variables|WFC|Sockets|GetNegYSocket)) (Utilities|String|EndsWith (Utilities|String|EnumtoString (Variables|WFC|Sockets|GetPosZSocket)) "S") (Utilities|String|EndsWith (Utilities|String|EnumtoString (Variables|WFC|Sockets|GetNegZSocket)) "S"))))